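; VisionPlace is an actor that cycles through alternative visions of a place, each made of world actors sharing a tag.
; NextVision advances a wrapping index, and Update shows and enables collision on actors with the current tag while hiding and disabling the others.
; A parallel rate array, filled with zeros (unset) on BeginPlay, stores a rate per vision through GetRate and SetRate for the current index.
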(event `self.ReceiveBeginPlay`
  (for _ (`self.VisionTags`)
    (`KismetArrayLibrary.Array_Add` (`self.VisionRates`)) ; Fill rates\n0 will mean unset
  )
  (`self.Update`))

(event `NextVision`
  (bind _result (`/Engine/EditorBlueprintResources/StandardMacros.IncrementInt` (`self.VisionIndex`))
    (:`  `
      (if (>= _result (`KismetArrayLibrary.Array_Length` (`self.VisionTags`)))
        (set `self.VisionIndex` 0))
      (`self.Update`))))

(fn `GetRate`
  (returns (rate :type Integer))
  (return (`|GetArrayItem` (`self.VisionRates`) (`self.VisionIndex`))))

(fn `SetRate`
  (params (rate :type Integer))
  (`KismetArrayLibrary.Array_Set` (`self.VisionRates`) (`self.VisionIndex`) rate))

(fn `Update`
  (for (_array_element _array_index) (`self.VisionTags`)
    (bind _outactors (`GameplayStatics.GetAllActorsWithTag` (`KismetStringLibrary.Conv_StringToName` _array_element)))
    (bind _returnvalue (== _array_index (`self.VisionIndex`)))
    (`self.SetActorHiddenInGame` _outactors (not _returnvalue))
    (`self.SetActorEnableCollision` _outactors _returnvalue)))

(fn `UserConstructionScript`)