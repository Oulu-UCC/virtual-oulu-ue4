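; AI character that wanders between the level's TargetPoints while its Tuntematonactor component turns to face the player.
; BeginPlay caches all TargetPoints as waypoints, and Tick sends the character to a random one with SimpleMoveToActor whenever its speed drops below a small threshold.
; Tick also sets that component's world rotation toward the first player's pawn.
; The construction script randomly picks a skeletal mesh, though every branch currently assigns SK_Mannequin.
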(event `self.ReceiveBeginPlay`
  (bind _outactors (`GameplayStatics.GetAllActorsOfClass` "/Script/Engine.TargetPoint"))
  (set `self.Waypoints` _outactors))

(event `self.ReceiveTick`
  (params (DeltaSeconds :type "Float (single-precision)"))
  (`|ExecutionSequence`
    (:`then_0`
      (if (not (>= (`KismetMathLibrary.VSize` (`MovementComponent.Velocity` (`self.CharacterMovement`))) 1.0))
        (`NavigationSystem.SimpleMoveToActor` (`self.GetController`) (`|GetArrayItem` (`self.Waypoints`) (`KismetMathLibrary.RandomInteger` (`KismetArrayLibrary.Array_Length` (`self.Waypoints`)))))))
    (:`then_1`
      (`SceneComponent.K2_SetWorldRotation` (`self.Tuntematonactor`) (`KismetMathLibrary.FindLookAtRotation` (`self.K2_GetActorLocation`) (`self.K2_GetActorLocation` (`GameplayStatics.GetPlayerPawn` 0))) false false))))

(fn `UserConstructionScript`
  (bind _mesh (`self.Mesh`))
  (switch `int` (`KismetMathLibrary.RandomInteger` 4)
    (:`0`
      (`SkinnedMeshComponent.SetSkinnedAssetAndUpdate` _mesh "/Game/Characters/Mannequin/Character/Mesh/SK_Mannequin.SK_Mannequin" true))
    (:`1`
      (`SkinnedMeshComponent.SetSkinnedAssetAndUpdate` _mesh "/Game/Characters/Mannequin/Character/Mesh/SK_Mannequin.SK_Mannequin" true))
    (:`2`
      (`SkinnedMeshComponent.SetSkinnedAssetAndUpdate` _mesh "/Game/Characters/Mannequin/Character/Mesh/SK_Mannequin.SK_Mannequin" true))
    (:`3`
      (`SkinnedMeshComponent.SetSkinnedAssetAndUpdate` _mesh "/Game/Characters/Mannequin/Character/Mesh/SK_Mannequin.SK_Mannequin" true))))