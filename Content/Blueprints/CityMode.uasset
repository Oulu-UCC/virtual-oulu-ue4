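; CityMode is a game mode that places the player at a named city spawn point when play begins.
; BeginPlay reads the "spawn" option from the options string, choosing between Kebabkuja, Rotuaari and Vaaranpuisto, or the first PlayerStart found by default.
; A helper finds the PlayerStart with the matching tag, and another teleports player pawn 0 to its location and rotation.
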(event `self.ReceiveBeginPlay`
  (switch `string` (`GameplayStatics.ParseOption` (`self.OptionsString`) "spawn")
    (:`Default`
      (bind _outactors (`GameplayStatics.GetAllActorsOfClass` "/Script/Engine.PlayerStart"))
      (`self.TeleportPlayerTo` (`|GetArrayItem` _outactors)))
    (:`Kebabkuja`
      (bind _start (`self.GetPlayerStartWithTag` "Kebabkuja"))
      (`self.TeleportPlayerTo` _start))
    (:`Rotuaari`
      (bind _start_2 (`self.GetPlayerStartWithTag` "Rotuaari"))
      (`self.TeleportPlayerTo` _start_2))
    (:`Vaaranpuisto`
      (bind _start_3 (`self.GetPlayerStartWithTag` "Vaaranpuisto"))
      (`self.TeleportPlayerTo` _start_3))))

(fn `UserConstructionScript`)